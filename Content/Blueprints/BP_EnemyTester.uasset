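; BP_EnemyTester is a test actor that repeatedly damages every BP_Enemy in the level, starting at BeginPlay.
; Each pass gathers the enemies with GetAllActorsOfClass, prints their count, and calls each one's TakeDamage event with a small random amount.
; It then prints a completion message and re-triggers its GiveDamage event after a short delay, forming an endless loop.
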(event Custom|Give%20Damage
  (bind _outactors (Actor|GetAllActorsOfClass "/Game/Blueprints/BP_Enemy.BP_Enemy_C")) ; Finds all of the enemies
  (Development|PrintString (Utilities|String|Append "There are " (Utilities|String|ToString(Integer) (Utilities|Array|Length _outactors)) "enemies in the level"))
  (for _array_element _outactors
    (Default|TakeDamage _array_element (Math|Random|RandomFloatinRange 0.1 0.5)) ; Custom Event from BP_enemy that gives the print string of ouch
  )
  (Development|PrintString "We've given damage to all of the enemies" true true "(R=0.000000,G=0.660000,B=1.000000,A=1.000000)" 5.0) ; Prints only when all the enemies have been afflicted. Should only play once
  (Utilities|FlowControl|Delay 2.0)
  (CallFunction|GiveDamage))

(event EventBeginPlay
  (bind _outactors (Actor|GetAllActorsOfClass "/Game/Blueprints/BP_Enemy.BP_Enemy_C")) ; Finds all of the enemies
  (Development|PrintString (Utilities|String|Append "There are " (Utilities|String|ToString(Integer) (Utilities|Array|Length _outactors)) "enemies in the level"))
  (for _array_element _outactors
    (Default|TakeDamage _array_element (Math|Random|RandomFloatinRange 0.1 0.5)) ; Custom Event from BP_enemy that gives the print string of ouch
  )
  (Development|PrintString "We've given damage to all of the enemies" true true "(R=0.000000,G=0.660000,B=1.000000,A=1.000000)" 5.0) ; Prints only when all the enemies have been afflicted. Should only play once
  (Utilities|FlowControl|Delay 2.0)
  (CallFunction|GiveDamage))

(fn ConstructionScript)