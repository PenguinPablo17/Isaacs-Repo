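; BP_Pickup is a carryable item actor with Pickup, Drop and PrimaryAction events.
; Pickup disables the Cube's collision and runs an attach to Pickup_Socket on the passed capsule component, snapping location and rotation.
; Drop restores collision, detaches the Cube, enables physics and tosses it with a fixed world-space force.
; PrimaryAction is a placeholder that only prints a debug message.
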(event Custom|Pickup
  (params (Capsule%20Component :type Scene%20Component%20Object%20Reference))
  (Development|PrintString "Pickup")
  (Collision|SetCollisionEnabled (Variables|Default|GetCube) "NoCollision")
  (Transformation|AttachComponentToComponent Capsule%20Component "Pickup_Socket" "SnapToTarget" "SnapToTarget" "KeepRelative" true))

(event Custom|Primary%20Action
  (Development|PrintString "Primary action"))

(event Custom|Drop
  (Development|PrintString "drop")
  (Collision|SetCollisionEnabled (Variables|Default|GetCube) "QueryAndPhysics")
  (Transformation|DetachFromComponent (Variables|Default|GetCube) "KeepRelative" "KeepRelative" "KeepRelative" true)
  (Physics|SetSimulatePhysics (Variables|Default|GetCube) true)
  (Physics|AddForce (Variables|Default|GetCube) "500.000000,0.000000,250.000000" "None" true))

(fn ConstructionScript)