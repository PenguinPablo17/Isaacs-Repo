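; BP_Enemy is a basic enemy actor that prints a greeting threat when play begins.
; A TakeDamage event prints a reaction and subtracts the incoming amount from Health.
; The CheckIfDead function tests whether Health is at or below zero, and the actor destroys itself when it is.
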(event Custom|Take%20Damage
  (params (By%20Ammounts :type Float%20%28double-precision%29))
  (Development|PrintString "Ouch")
  (Variables|Default|SetHealth (- (Variables|Default|GetHealth) By%20Ammounts))
  (if (CallFunction|CheckifDead (Variables|Default|GetHealth))
    (Actor|DestroyActor)))

(event EventBeginPlay
  (Development|PrintString "Aloha friend. Prepare to die."))

(fn ConstructionScript)

(fn CheckifDead
  (params (Health :type Float%20%28double-precision%29))
  (return (<= Health 0.0)))